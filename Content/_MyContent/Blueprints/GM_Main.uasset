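; GM_Main is the manager for a 60-second clicker game where clicks raise levels and fans, but clicking while PARYI is inside risks a bad ending.
; BeginPlay caches scene actors, creates menu and HUD widgets, and loads or creates the save.
; A one-second timer tries the door, computes clicks per second to drive MEA's play rate, adds fans and judges the ending at timeout.
; It also handles settings pause, input modes and effects volume.
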(event `self.ReceiveBeginPlay`
  (bind _returnvalue (`GameUserSettings.GetGameUserSettings`))
  (`GameUserSettings.SetScreenResolution` _returnvalue (make `IntPoint` 1280 720))
  (`GameUserSettings.ApplySettings` _returnvalue true)
  (bind _aspc_player_controller (cast `/Game/_MyContent/Blueprints/PC_PlayerController` (`GameplayStatics.GetPlayerController` 0)))
  (bind _output_get (set `self.REF_PC` _aspc_player_controller))
  (`|ExecutionSequence`
    (:`then_0`
      (`self.InitGetSceneObjs`) ; Init Get Scene Objs
    )
    (:`then_1`
      (bind _returnvalue_2 (`|CreateWidget` "/Game/_MyContent/Blueprints/WB_StartMenu.WB_StartMenu_C"))
      (`UserWidget.AddToViewport` _returnvalue_2 0))
    (:`then_2`
      (bind (_asbp_setting_save _isnewdata) (`self.LoadGameData`))
      (if _isnewdata
        (bind _returnvalue_3 (`|CreateWidget` "/Game/_MyContent/Blueprints/WB_Setting.WB_Setting_C" _output_get))
        (`UserWidget.AddToViewport` _returnvalue_3 0)))
    (:`then_3`
      (bind _returnvalue_4 (`|CreateWidget` "/Game/_MyContent/Blueprints/WB_GUI.WB_GUI_C" _output_get))
      (bind _output_get_2 (set `self.REF_WB_GUI` _returnvalue_4))
      (`UserWidget.AddToViewport` _output_get_2 0)
      (`Widget.SetVisibility` _output_get_2 "Hidden"))
    (:`then_4`
      (`self.SwitchMouseInputMode` true)
      ;[1 1 1] SpawnClickSound
      (bind _returnvalue_5 (`GameplayStatics.SpawnSound2D` "/Game/_MyContent/Sounds/laugh.laugh" 1.0 1.0 0.0 null false false))
      (bind _output_get_3 (set `self.ClickSound` _returnvalue_5))
      (`AudioComponent.Stop` _output_get_3))))

(event `OnGameStart`
  ;[1 1 1] GameStart
  (`self.SwitchMouseInputMode` false)
  (`/Game/_MyContent/Blueprints/WB_GUI.OnGameStart` (`self.REF_WB_GUI`))
  (`self.GameStartOP`))

(event `OnGameEnd`
  (params (IsGoodEnd :type Boolean))
  ;[1 1 1] GameEnd
  (`self.SwitchMouseInputMode` true)
  (`/Game/_MyContent/Blueprints/WB_GUI.OnGameEnd` (`self.REF_WB_GUI`) IsGoodEnd)
  (`self.GameEndOP`)
  (if (not IsGoodEnd)
    ;;[1 1 1] EndSound
    (`AudioComponent.Stop` (`self.ClickSound`))
    (`GameplayStatics.PlaySound2D` "/Game/_MyContent/Sounds/Scream_Cue.Scream_Cue")))

(event `OnScreenClick`
  ;[1 1 1] OnGameClick
  (if (`self.IsGameGoning`)
    (`|ExecutionSequence`
      (:`then_0`
        (`self.PlayClickSound`))
      (:`then_1`
        (`self.PlayClickAni`))
      (:`then_2`
        (if (`self.Is_PARYI_Inside`)
          (`/Game/_MyContent/Blueprints/WB_GUI.PlayPB_BAD_Ani` (`self.REF_WB_GUI`))
          (`/Game/_MyContent/Blueprints/BP_Door.PlayParyiHitAni` (`self.REF_BP_Door`))
          (`/Game/_MyContent/Blueprints/BP_MEA.PlayHitAni` (`self.REF_PF_MEA`))
          (bind _result (`/Engine/EditorBlueprintResources/StandardMacros.IncrementInt` (`self.SawFAPTimes`))
            (:`  `
              (if (> _result (`self.SawCanFTimes`))
                (`self.OnGameEnd` false))))
          (else
            (`self.AddClickTimes`)
            (`self.AddProgress`)
            (`self.AddLevel`)
            (`self.AddFansNums`)))))))

(event `OnSEVolumeChange`
  (params (Volume :type "Float (double-precision)") (IsPlaySound :type Boolean))
  (`GameplayStatics.SetSoundMixClassOverride` (`self.REF_SESoundMixer`) "/Game/_MyContent/Sounds/SE_SoundClass.SE_SoundClass" Volume)
  (if IsPlaySound
    (`GameplayStatics.PlaySound2D` "/Game/_MyContent/Sounds/nihao_Cue.nihao_Cue")))

(fn `AddClickTimes`
  (`/Engine/EditorBlueprintResources/StandardMacros.IncrementInt` (`self.ClickTimes`)))

(fn `AddFansNums`
  (bind _output_get (set `self.CurAddFansNums` (+ (* (`self.CurLevel`) (`KismetMathLibrary.RandomIntegerInRange` 5 30)) (`KismetMathLibrary.FTrunc` (`self.CPS`)))))
  (set `self.FansNums` (+ (`self.FansNums`) _output_get)))

(fn `AddLevel`
  (if (>= (`KismetMathLibrary.Conv_IntToDouble` (`self.CurLevelClickTimes`)) (`self.LevelUpCount`))
    (set `self.CurLevelClickTimes` 0)
    (`/Engine/EditorBlueprintResources/StandardMacros.IncrementInt` (`self.CurLevel`)
      (:`  `
        (set `self.LevelUpCount` (* (`self.LevelUpCount`) (`self.LevelUpCountIncrease`)))))
    (else
      (`/Engine/EditorBlueprintResources/StandardMacros.IncrementInt` (`self.CurLevelClickTimes`)))))

(fn `AddProgress`
  (set `self.CurPercent` (/ (`KismetMathLibrary.Conv_IntToDouble` (`self.CurLevelClickTimes`)) (`self.LevelUpCount`))))

(fn `ComputeCPS`
  (bind _clicktimes (`self.ClickTimes`))
  (bind _cps (`self.CPS`))
  (set `self.CPS` (`KismetMathLibrary.Conv_IntToDouble` (- _clicktimes (`self.LastClickTimes`))))
  (set `self.LastClickTimes` _clicktimes)
  (`PaperFlipbookComponent.SetPlayRate` (`PaperFlipbookActor.RenderComponent` (`self.REF_PF_MEA`)) (* (`KismetMathLibrary.FClamp` _cps 0.3 _cps) 0.9)))

(fn `GameEndOP`
  (set `self.IsGameGoning` false)
  (`PaperFlipbookComponent.SetPlayRate` (`PaperFlipbookActor.RenderComponent` (`self.REF_PF_MEA`)) 0.0)
  (`KismetSystemLibrary.K2_ClearAndInvalidateTimerHandle` (`self.CountdownTimerHandle`))
  (`self.GameEnded`))

(fn `GameStartOP`
  (`/Game/_MyContent/Blueprints/BP_Door.Init` (`self.REF_BP_Door`))
  (bind _returnvalue (`KismetSystemLibrary.K2_SetTimer` null "TimerCountDown" 1.0 true))
  (set `self.CountdownTimerHandle` _returnvalue)
  (`|ExecutionSequence`
    (:`then_0`
      (set `self.FansNums` 0)
      (set `self.IsGameGoning` true))
    (:`then_1`
      (set `self.CurLevel` 0)
      (set `self.CurLevelClickTimes` 0))
    (:`then_2`
      (set `self.CPS` 0.0)
      (set `self.SawFAPTimes` 0))
    (:`then_3`
      (set `self.CurPercent` 0.0)
      (set `self.LastLevel` -1) ; Last Need to -1
    )
    (:`then_4`
      (set `self.ClickTimes` 0)
      (set `self.TimeLeft` 60))
    (:`then_5`
      (set `self.LastClickTimes` 0)
      (set `self.LevelUpCount` 2.0)
      (set `self.CurAddFansNums` 0))
    (:`then_6`
      (`self.GameStarted`))))

(fn `InitGetSceneObjs`
  (`|ExecutionSequence`
    (:`then_0`
      (bind _outactors (`GameplayStatics.GetAllActorsWithTag` "SpawnPoint"))
      (set `self.REF_SpawnsPointsArr` _outactors))
    (:`then_1`
      (bind _outactors_2 (`GameplayStatics.GetAllActorsOfClass` "/Game/_MyContent/Blueprints/BP_Desk.BP_Desk_C"))
      (set `self.REF_BP_Desk` (`|GetArrayItem` _outactors_2)))
    (:`then_2`
      (bind _outactors_3 (`GameplayStatics.GetAllActorsOfClass` "/Game/_MyContent/Blueprints/BP_Door.BP_Door_C"))
      (set `self.REF_BP_Door` (`|GetArrayItem` _outactors_3)))
    (:`then_3`
      (bind _outactors_4 (`GameplayStatics.GetAllActorsOfClass` "/Game/_MyContent/Blueprints/BP_MEA.BP_MEA_C"))
      (set `self.REF_PF_MEA` (`|GetArrayItem` _outactors_4)))))

(fn `LoadGameData`
  (returns (`AsBP Setting Save` :type "/Game/_MyContent/Blueprints/BP_GameSave Object Reference") (IsNewData :type Boolean))
  (bind _returnvalue (`GameplayStatics.LoadGameFromSlot` "MyGameSave"))
  (bind _asbp_game_save (cast `/Game/_MyContent/Blueprints/BP_GameSave` _returnvalue)
    (:`then`
      (return _asbp_game_save false))
    (:`CastFailed`
      (bind _returnvalue_2 (`GameplayStatics.CreateSaveGameObject` "/Game/_MyContent/Blueprints/BP_GameSave.BP_GameSave_C"))
      (`self.SaveGameData` _returnvalue_2)
      (return _returnvalue_2 true))))

(fn `OpenTheDoor`
  (if (not (`self.Is_PARYI_Inside`))
    (`/Game/_MyContent/Blueprints/BP_Door.TryToOpenTheDoor` (`self.REF_BP_Door`))))

(fn `PlayClickAni`
  (bind _ref_wb_gui (`self.REF_WB_GUI`))
  (`|ExecutionSequence`
    (:`then_0`
      (if (`self.Is_PARYI_Inside`)
        (`/Game/_MyContent/Blueprints/WB_GUI.PlayPB_BAD_Ani` _ref_wb_gui)
        (else
          (`/Game/_MyContent/Blueprints/WB_GUI.PlayPB_OK_Ani` _ref_wb_gui))))
    (:`then_1`
      (`/Game/_MyContent/Blueprints/BP_Desk.PlayF*pAni` (`self.REF_BP_Desk`)))))

(fn `PlayClickSound`
  (if (`self.Is_PARYI_Inside`)
    _
    (else
      _))
  (`AudioComponent.Play` (`self.ClickSound`) 0.0))

(fn `SaveGameData`
  (params (SaveGameObject :type "SaveGame Object Reference"))
  (`GameplayStatics.SaveGameToSlot` SaveGameObject "MyGameSave"))

(fn `ShowSettingWB`
  (params (IsSettingOpen :type Boolean))
  (bind _ref_wb_settings (`self.REF_WB_Settings`))
  (bind _ref_wb_settings_2 (`self.REF_WB_Settings`))
  (`GameplayStatics.SetGamePaused` IsSettingOpen)
  (if IsSettingOpen
    (`/Engine/EditorBlueprintResources/StandardMacros.IsValid` _ref_wb_settings_2
      (:`Is Valid`
        (`UserWidget.AddToViewport` _ref_wb_settings_2 0))
      (:`Is Not Valid`
        (bind _returnvalue (`|CreateWidget` "/Game/_MyContent/Blueprints/WB_Setting.WB_Setting_C" (`self.REF_PC`)))
        (bind _output_get (set `self.REF_WB_Settings` _returnvalue))
        (`UserWidget.AddToViewport` _output_get 0)))
    (else
      (`/Engine/EditorBlueprintResources/StandardMacros.IsValid` _ref_wb_settings
        (:`Is Valid`
          (`Widget.RemoveFromParent` _ref_wb_settings))))))

(fn `SwitchMouseInputMode`
  (params (IsUIInput :type Boolean))
  (bind _ref_pc (`self.REF_PC`))
  (if IsUIInput
    (`WidgetBlueprintLibrary.SetInputMode_UIOnlyEx` _ref_pc)
    (set `PlayerController.bShowMouseCursor` true _ref_pc)
    (else
      (`WidgetBlueprintLibrary.SetInputMode_GameAndUIEx` _ref_pc null "DoNotLock" false)
      (set `PlayerController.bShowMouseCursor` true _ref_pc)))
  (return))

(fn `TimerCountDown`
  (`self.OpenTheDoor`)
  (`self.ComputeCPS`)
  (`self.AddFansNums`)
  (bind _result (`/Engine/EditorBlueprintResources/StandardMacros.DecrementInt` (`self.TimeLeft`))
    (:`  `
      (if (< _result 0)
        (set `self.TimeLeft` 0)
        (`self.OnGameEnd` (>= (`self.FansNums`) 20000))))))

(fn `UserConstructionScript`)