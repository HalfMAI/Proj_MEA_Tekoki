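; BP_Door is a door that randomly rattles its handle and sometimes opens, setting the GM_Main flag IsPARYIInside while it does.
; TryToOpenTheDoor passes a coin flip and busy guard, plays the handle sequence, then opens with a chance that rises with CurLevel.
; Level sequence players drive the motion at random speeds with random delays, reversing the door sequence to close before clearing both flags.
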(event `self.ReceiveBeginPlay`
  (bind _asgm_main (cast `/Game/_MyContent/Blueprints/GM_Main` (`GameplayStatics.GetGameMode`)))
  (set `self.REG_GM` _asgm_main)
  (`self.Init`))

(event `TryToOpenTheDoor`
  (bind _reg_gm (`self.REG_GM`))
  (if (`self.IsDoorActioning`)
    _
    (elif (`KismetMathLibrary.RandomBool`)
      (set `self.IsDoorActioning` true)
      (`self.PlayHandleAni`)
      (`KismetSystemLibrary.Delay` (`KismetMathLibrary.RandomFloatInRange` 0.5 1.0))
      (if (< (`KismetMathLibrary.RandomFloatInRange` 0.0 1.0) (* (`/Game/_MyContent/Blueprints/GM_Main.CurLevel` _reg_gm) 0.15))
        (set `/Game/_MyContent/Blueprints/GM_Main.Is_PARYI_Inside` true _reg_gm)
        (`self.PlayDoorOpenAni`)
        (`KismetSystemLibrary.Delay` (`KismetMathLibrary.RandomFloatInRange` 1.0 3.0))
        (`self.PlayDoorCloseAni`)
        (`KismetSystemLibrary.Delay` 1.0))
      (set `self.IsDoorActioning` false)
      (set `/Game/_MyContent/Blueprints/GM_Main.Is_PARYI_Inside` false _reg_gm))))

(fn `Init`
  (set `self.IsDoorActioning` false)
  (`MovieSceneSequencePlayer.SetPlaybackPosition` (`ActorSequenceComponent.SequencePlayer` (`self.DoorOpenSeq`)) 0.0))

(fn `PlayDoorCloseAni`
  (bind _sequenceplayer (`ActorSequenceComponent.SequencePlayer` (`self.DoorOpenSeq`)))
  (`MovieSceneSequencePlayer.SetPlaybackPosition` _sequenceplayer 1.0)
  (`MovieSceneSequencePlayer.PlayReverse` _sequenceplayer))

(fn `PlayDoorOpenAni`
  (bind _sequenceplayer (`ActorSequenceComponent.SequencePlayer` (`self.DoorOpenSeq`)))
  (`MovieSceneSequencePlayer.SetPlayRate` _sequenceplayer (`KismetMathLibrary.RandomFloatInRange` 0.5 1.5))
  (`MovieSceneSequencePlayer.SetPlaybackPosition` _sequenceplayer 0.0)
  (`MovieSceneSequencePlayer.Play` _sequenceplayer)
  (`GameplayStatics.PlaySound2D` "/Game/_MyContent/Sounds/nihao.nihao"))

(fn `PlayHandleAni`
  (bind _sequenceplayer (`ActorSequenceComponent.SequencePlayer` (`self.HandleOpenSeq`)))
  (`MovieSceneSequencePlayer.SetPlayRate` _sequenceplayer (`KismetMathLibrary.RandomFloatInRange` 0.5 1.5))
  (`MovieSceneSequencePlayer.SetPlaybackPosition` _sequenceplayer 0.0)
  (`MovieSceneSequencePlayer.Play` _sequenceplayer))

(fn `UserConstructionScript`)