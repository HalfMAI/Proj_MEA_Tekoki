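; Player controller that forwards click and pause-style key input to the GM_Main game mode.
; On BeginPlay it caches the game mode and binds to its game started and ended events to track whether play is active.
; Left mouse and Space both trigger the screen click action.
; Escape and Q toggle the settings widget through a FlipFlop, only while the game is started.
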(event `self.ReceiveBeginPlay`
  (bind _asgm_main (cast `/Game/_MyContent/Blueprints/GM_Main` (`GameplayStatics.GetGameMode`)))
  (bind _output_get (set `self.REF_Main_GameMode` _asgm_main))
  (add `/Game/_MyContent/Blueprints/GM_Main.GameStarted` _output_get (delegate `OnGameStarted`))
  (add `/Game/_MyContent/Blueprints/GM_Main.GameEnded` _output_get (delegate `OnGameEnded`)))

(event `OnGameStarted`
  (set `self.IsGameStarted` true))

(event `OnGameEnded`
  (set `self.IsGameStarted` false))

(event `Key|LeftMouseButton`
  (params (Key :type "Key Structure"))
  (:`Pressed`
    (`/Game/_MyContent/Blueprints/GM_Main.OnScreenClick` (`self.REF_Main_GameMode`) :!label _label)))

(event `Key|SpaceBar`
  (params (Key :type "Key Structure"))
  (:`Pressed`
    (goto _label)))

(event `Key|Escape` :paused true
  (params (Key :type "Key Structure"))
  (:`Pressed`
    (if (`self.IsGameStarted`) :!label _label_2
      (bind _isa (`/Engine/EditorBlueprintResources/StandardMacros.FlipFlop`)
        (:`A`
          _)
        (:`B`
          _))
      (`/Game/_MyContent/Blueprints/GM_Main.ShowSettingWB` (`self.REF_Main_GameMode`) _isa))))

(event `Key|Q` :paused true
  (params (Key :type "Key Structure"))
  (:`Pressed`
    (goto _label_2)))

(fn `UserConstructionScript`)