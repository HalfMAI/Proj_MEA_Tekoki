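; BP_Desk is a desk actor that gives animated feedback showing the current fan gain.
; On BeginPlay it caches the GM_Main game mode.
; PlayFpAni restarts the FpAni sequence from the beginning and spawns a BP_FloatingStrings at SpawnPoint, setting its text to a plus sign and the game mode's CurAddFansNums.
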(event `self.ReceiveBeginPlay`
  (bind _asgm_main (cast `/Game/_MyContent/Blueprints/GM_Main` (`GameplayStatics.GetGameMode`)))
  (set `self.REF_GM` _asgm_main))

(fn `PlayF*pAni`
  (bind _sequenceplayer (`ActorSequenceComponent.SequencePlayer` (`self.F*pAni`)))
  (`MovieSceneSequencePlayer.SetPlaybackPosition` _sequenceplayer 0.0)
  (`MovieSceneSequencePlayer.Play` _sequenceplayer)
  (bind _returnvalue (`|SpawnActorFromClass` "/Game/_MyContent/Blueprints/BP_FloatingStrings.BP_FloatingStrings_C" (`SceneComponent.K2_GetComponentToWorld` (`self.SpawnPoint`)) "Undefined" "OverrideRootScale" null null))
  (`TextRenderComponent.K2_SetText` (`TextRenderActor.TextRender` _returnvalue) (`|FormatText` "+{Num}" (`/Game/_MyContent/Blueprints/GM_Main.CurAddFansNums` (`self.REF_GM`)))))

(fn `UserConstructionScript`)